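; BP_TargetHit is a damageable target that slides side to side and shows a health bar.
; Tick oscillates the Box's relative Y with a sine wave, using its starting Y as a time offset.
; Health getters, Heal and TakeDamage forward to BPCHealthSystem, and the healthbar widget receives the actor as its DamagableActor.
; The construction script binds the component's death, block and damage events, whose handlers only print debug messages.
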(event `self.ReceiveBeginPlay`
  (bind _returnvalue_location (`KismetMathLibrary.BreakTransform` (`SceneComponent.GetRelativeTransform` (`self.Box`))))
  (`|ExecutionSequence`
    (:`then_0`
      (set `self.Location` _returnvalue_location))
    (:`then_1`
      (bind _returnvalue (`|CreateWidget` "/Game/HealthSystem/Healthbar/W_Healthbar.W_Healthbar_C" null self))
      (`WidgetComponent.SetWidget` (`self.Widget`) _returnvalue))))

(event `self.ReceiveTick`
  (params (DeltaSeconds :type "Float (single-precision)"))
  (bind (_location_x _location_y _location_z) (`KismetMathLibrary.BreakVector` (`self.Location`)))
  (`SceneComponent.K2_SetRelativeLocation` (`self.Box`) (`KismetMathLibrary.MakeVector` _location_x (* (`KismetMathLibrary.DegSin` (* (+ (`self.GetGameTimeSinceCreation`) _location_y) (`self.Speed`))) (`self.Distance`)) _location_z) false false))

(event `OnDeath`
  (`KismetSystemLibrary.PrintString` "Dead"))

(event `OnBlocked`
  (params (canBeParried :type Boolean))
  (`KismetSystemLibrary.PrintString` (`KismetStringLibrary.BuildString_Bool` "OnBlocked, " "can be parried" canBeParried)))

(event `OnDamageRecieved`
  (bind _currenthealth (`self.GetCurrentHealth`))
  (`KismetSystemLibrary.PrintString` (`KismetStringLibrary.BuildString_Double` "" "Health: " _currenthealth)))

(fn `GetCurrentHealth`
  (returns (CurrentHealth :type "Float (double-precision)"))
  (bind _currenthealth (`/Game/HealthSystem/BPC_HealthSystem.GetCurrentHealth` (`self.BPC_HealthSystem`)))
  (return _currenthealth))

(fn `GetMaxHealth`
  (returns (MaxHealth :type "Float (double-precision)"))
  (bind _maxhealth (message `/Game/HealthSystem/BPI_Damagable.GetMaxHealth` (`self.BPC_HealthSystem`)))
  (return _maxhealth))

(fn `Heal`
  (params (Amount :type "Float (double-precision)"))
  (returns (Health :type "Float (double-precision)"))
  (bind _health (`/Game/HealthSystem/BPC_HealthSystem.Heal` (`self.BPC_HealthSystem`) Amount))
  (return _health))

(fn `TakeDamage`
  (params (DamageInfo :type "/Game/HealthSystem/Structures/DamageInfo_Struct Structure"))
  (returns (IsDamaged :type Boolean))
  (bind _isdamaged (`/Game/HealthSystem/BPC_HealthSystem.Damage` (`self.BPC_HealthSystem`) DamageInfo))
  (return _isdamaged))

(fn `UserConstructionScript`
  (bind _bpc_healthsystem (`self.BPC_HealthSystem`))
  (`|ExecutionSequence`
    (:`then_0`
      (add `/Game/HealthSystem/BPC_HealthSystem.OnDeath` _bpc_healthsystem (`|CreateDelegate` :!event `OnDeath`)))
    (:`then_1`
      (add `/Game/HealthSystem/BPC_HealthSystem.OnBlocked` _bpc_healthsystem (`|CreateDelegate` :!event `OnBlocked`)))
    (:`then_2`
      (add `/Game/HealthSystem/BPC_HealthSystem.OnDamaged` _bpc_healthsystem (`|CreateDelegate` :!event `OnDamageRecieved`)))))